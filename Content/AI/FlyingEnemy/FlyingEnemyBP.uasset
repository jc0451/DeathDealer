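; Flying enemy Blueprint that hooks an AI-controlled enemy up to its behavior tree and damage system.
; The construction script initializes its DamageComponent with the enemy's max HP as both maximum and starting health.
; On BeginPlay it casts its controller to MyAI and passes in the behavior tree and the player pawn as the sensing target.
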(event EventBeginPlay
  (bind _asmy_ai (Utilities|Casting|CastToMyAI (AI|GetAIController self)))
  (Default|SetupAIC _asmy_ai (Variables|Default|GetBT) (Game|Player|GetPlayerPawn 0)))

(fn ConstructionScript
  (bind _flyingenemymaxhp (Variables|Default|GetFlyingEnemyMaxHP))
  (Default|SetupDamageComponent (Variables|Default|GetDamageComponent) self _flyingenemymaxhp _flyingenemymaxhp))